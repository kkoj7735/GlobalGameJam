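; Example NPC supporting interactive dialogue and non-interactive self-talk, the latter triggered by a large sphere overlap.
; Two dialogue components play animation, voice and subtitles from data table rows keyed by a shared SaveScene name.
; Interactive dialogue can instead play an async-loaded Level Sequence, though BeginPlay selects AnimVoice.
; Finishing a line increments the row name's numeric suffix, while hard-coded cases handle scene ends, options and skips.
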(event OnComponentBeginOverlap(LargeSphere(fornon-interactive))
  (params (OverlappedComponent :type Primitive%20Component%20Object%20Reference) (OtherActor :type Actor%20Object%20Reference) (OtherComp :type Primitive%20Component%20Object%20Reference) (OtherBodyIndex :type Integer) (bFromSweep :type Boolean) (SweepResult :type Hit%20Result%20Structure%20%28by%20ref%29))
  ;[1 1 1] Example of a scene dialogue [Non-Interactive]
  (if (Utilities|DoesObjectImplementInterface OtherActor "/Game/Luxuanlin/DialogueSystem/BP_Interface/BPI_NonInteractiveInterface.BPI_NonInteractiveInterface_C") ; Add more condition to verify if player is busy
    (Utilities|Casting|CastToSphereComponent OtherComp) ; if main character using a sphere detection
    (Default|StartSelfTalk(Non-Interactive) (Variables|Default|GetBPac_Dialogue_NonInteractive) "NewEnumerator0")))

(event EventBeginPlay
  ;[1 1 1] Begin
  (Variables|/Game/Luxuanlin/DialogueSystem/ActorComponent_Dialogue/BPac_Dialogue.BPac_Dialogue_C|SetNPC_Mesh (Variables|Default|GetBPac_Dialogue) (Variables|Character|GetMesh))
  (Variables|/Game/Luxuanlin/DialogueSystem/ActorComponent_Dialogue/BPac_Dialogue_NonInteractive.BPac_Dialogue_NonInteractive_C|SetNPC_Mesh (Variables|Default|GetBPac_Dialogue_NonInteractive) (Variables|Character|GetMesh))
  (Variables|Default|SetSaveScene "Scene1.0")
  (Variables|Default|SetSaveCinematic "Cine1.0")
  (Variables|Default|SetTypeScene "AnimVoice"))

(event EventFinishedDialogue(Non-Interactive)
  ;[1 1 1] Example of Finished dialogue [Non-Interactive]
  (bind _returnvalue (Class|DataTableFunctionLibrary|DoesDataTableRowExist "/Game/Luxuanlin/DialogueSystem/Characters/DataTable/DT_Dialogue_A.DT_Dialogue_A" (Utilities|String|StringToName (Utilities|String|BuildString(Integer) (.LeftS (Utilities|String|Split (Utilities|String|ToString(Name) (Variables|Default|GetSaveScene)) "." "IgnoreCase" "FromEnd")) "." (+ (Math|Conversions|ToInteger(Byte) (.RightS (Utilities|String|Split (Utilities|String|ToString(Name) (Variables|Default|GetSaveScene)) "." "IgnoreCase" "FromEnd"))) 1)))))
  (if _returnvalue
    (Variables|Default|SetSaveScene (Utilities|String|StringToName (Utilities|String|BuildString(Integer) (.LeftS (Utilities|String|Split (Utilities|String|ToString(Name) (Variables|Default|GetSaveScene)) "." "IgnoreCase" "FromEnd")) "." (+ (Math|Conversions|ToInteger(Byte) (.RightS (Utilities|String|Split (Utilities|String|ToString(Name) (Variables|Default|GetSaveScene)) "." "IgnoreCase" "FromEnd"))) 1))))
    (Default|StartSelfTalk(Non-Interactive) (Variables|Default|GetBPac_Dialogue_NonInteractive) "NewEnumerator0")
    (else
      (switch name (Variables|Default|GetSaveScene)
        (:Scene1.9
          (Variables|Default|SetSaveScene "None"))))))

(event EventStartDialogue(Non-Interactive)
  (params (Action :type ENonIteractiveAction%20Enum :default "NewEnumerator0"))
  ;[1 1 1] Example of a scene dialogue [Non-Interactive]
  (switch Utilities|FlowControl|Switch|SwitchonENonIteractiveAction Action
    (:NewEnumerator0
      (bind _returnvalue (Utilities|GetDataTableRow "/Game/Luxuanlin/DialogueSystem/Characters/DataTable/DT_DialogueAnim_A.DT_DialogueAnim_A" (Variables|Default|GetSaveScene))
        (:then
          (Default|PlayAnimandVoice (Variables|Default|GetBPac_Dialogue_NonInteractive) _returnvalue)
          (bind _returnvalue_2 (Utilities|GetDataTableRow "/Game/Luxuanlin/DialogueSystem/Characters/DataTable/DT_Dialogue_A.DT_Dialogue_A" (Variables|Default|GetSaveScene))
            (:then
              (Default|DisplayText (Variables|/Game/Luxuanlin/DialogueSystem/ActorComponent_Dialogue/BPac_Dialogue_NonInteractive.BPac_Dialogue_NonInteractive_C|GetDialogueNonInteractiveUI (Variables|Default|GetBPac_Dialogue_NonInteractive)) _returnvalue_2))))))))

(event EventFinishedDialogue
  ;[1 1 1] Example of Finished/Skip/Option dialogue
  (bind _returnvalue (Class|DataTableFunctionLibrary|DoesDataTableRowExist "/Game/Luxuanlin/DialogueSystem/Characters/DataTable/DT_Dialogue_A.DT_Dialogue_A" (Utilities|String|StringToName (Utilities|String|BuildString(Integer) (.LeftS (Utilities|String|Split (Utilities|String|ToString(Name) (Variables|Default|GetSaveScene)) "." "IgnoreCase" "FromEnd")) "." (+ (Math|Conversions|ToInteger(Byte) (.RightS (Utilities|String|Split (Utilities|String|ToString(Name) (Variables|Default|GetSaveScene)) "." "IgnoreCase" "FromEnd"))) 1)))))
  (if _returnvalue
    (Variables|Default|SetSaveScene (Utilities|String|StringToName (Utilities|String|BuildString(Integer) (.LeftS (Utilities|String|Split (Utilities|String|ToString(Name) (Variables|Default|GetSaveScene)) "." "IgnoreCase" "FromEnd")) "." (+ (Math|Conversions|ToInteger(Byte) (.RightS (Utilities|String|Split (Utilities|String|ToString(Name) (Variables|Default|GetSaveScene)) "." "IgnoreCase" "FromEnd"))) 1))))
    (Class|BPIInteractTalkInterface|StartTalk(Message) (Variables|Default|GetBPac_Dialogue))
    (else
      (switch name (Variables|Default|GetSaveScene)
        (:Scene1.9
          (Variables|Default|SetSaveScene "Scene2.0"))
        (:Scene2.9
          (Variables|Default|SetSaveScene "Scene3.0"))))))

(event EventSelectedOption
  (params (OptionText :type Text))
  ;[1 1 1] Example of Finished/Skip/Option dialogue
  (switch name (Variables|Default|GetSaveScene)
    (:Scene1.1
      (switch string (Utilities|String|ToString(Text) OptionText)
        (:Yes
          (Variables|Default|SetSaveScene "Scene2.0")
          (Class|BPIInteractTalkInterface|StartTalk(Message) (Variables|Default|GetBPac_Dialogue)))))))

(event EventStartDialogue
  ;[1 1 1] Example of scene dialogue
  (switch name (Variables|Default|GetTypeScene)
    (:AnimVoice
      (bind _returnvalue (Utilities|GetDataTableRow "/Game/Luxuanlin/DialogueSystem/Characters/DataTable/DT_DialogueAnim_A.DT_DialogueAnim_A" (Variables|Default|GetSaveScene))
        (:then
          (Default|PlayAnimandVoice (Variables|Default|GetBPac_Dialogue) _returnvalue)
          (bind _returnvalue_2 (Utilities|GetDataTableRow "/Game/Luxuanlin/DialogueSystem/Characters/DataTable/DT_Dialogue_A.DT_Dialogue_A" (Variables|Default|GetSaveScene))
            (:then
              (Default|DisplayText (Variables|/Game/Luxuanlin/DialogueSystem/ActorComponent_Dialogue/BPac_Dialogue.BPac_Dialogue_C|GetDialogueUI (Variables|Default|GetBPac_Dialogue)) _returnvalue_2))))))
    (:Cinematic
      (Input|SetIgnoreLookInput (Game|GetPlayerController 0) true)
      (if (not (Variables|Default|GetbSequencerLoading)) ; still loading
        (bind _returnvalue_3 (Utilities|GetDataTableRow "/Game/Luxuanlin/DialogueSystem/Sequencer/DT_Sequencer.DT_Sequencer" (Variables|Default|GetSaveCinematic))
          (:then
            (Utilities|IsValid (Utilities|ResolveSoftReference (.levelsequence _returnvalue_3)) ; is already loaded
              (:Is%20Valid
                (Variables|Default|SetbSequencerLoading false :!label _label)
                (Default|PlaySequencer (Variables|Default|GetBPac_Dialogue) (Utilities|ResolveSoftReference (.levelsequence _returnvalue_3)))
                (bind _returnvalue_4 (Utilities|GetDataTableRow "/Game/Luxuanlin/DialogueSystem/Characters/DataTable/DT_Dialogue_A.DT_Dialogue_A" (Variables|Default|GetSaveScene))
                  (:then
                    (Default|DisplayText (Variables|/Game/Luxuanlin/DialogueSystem/ActorComponent_Dialogue/BPac_Dialogue.BPac_Dialogue_C|GetDialogueUI (Variables|Default|GetBPac_Dialogue)) _returnvalue_4))))
              (:Is%20Not%20Valid
                (Utilities|AsyncLoadAsset (.levelsequence _returnvalue_3)
                  (:then
                    (Variables|Default|SetbSequencerLoading true))
                  (:Completed
                    (goto _label)))))))))))

(event EventSkipDialogue
  ;[1 1 1] Example of Finished/Skip/Option dialogue
  (switch name (Utilities|String|StringToName (.LeftS (Utilities|String|Split (Utilities|String|ToString(Name) (Variables|Default|GetSaveScene)) "." "IgnoreCase" "FromEnd")))
    (:Scene1
      (Variables|Default|SetSaveScene "Scene2.0")
      (Class|BPIInteractTalkInterface|StartTalk(Message) (Variables|Default|GetBPac_Dialogue)))))

(fn ConstructionScript)

(fn GetInteractType
  (return (Variables|Default|GetInteract%20Type)))