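; Example non-interactive NPC that plays a scene of self-talk dialogue when a player-side actor enters its box.
; The overlap requires the non-interactive interface and a sphere component, then starts the dialogue component.
; The start event looks up SaveScene in two data tables to play animation and voice and display text.
; When a line finishes, it increments the row name's numeric suffix and continues while that row exists.
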(event OnComponentBeginOverlap(Box)
  (params (OverlappedComponent :type Primitive%20Component%20Object%20Reference) (OtherActor :type Actor%20Object%20Reference) (OtherComp :type Primitive%20Component%20Object%20Reference) (OtherBodyIndex :type Integer) (bFromSweep :type Boolean) (SweepResult :type Hit%20Result%20Structure%20%28by%20ref%29))
  ;[1 1 1] Example of a scene dialogue flow
  (if (Utilities|DoesObjectImplementInterface OtherActor "/Game/Luxuanlin/DialogueSystem/BP_Interface/BPI_NonInteractiveInterface.BPI_NonInteractiveInterface_C") ; Add more condition to verify if player is busy
    (Utilities|Casting|CastToSphereComponent OtherComp) ; to differenciate between the collision of the sphere or the capsule
    (Default|StartSelfTalk(Non-Interactive) (Variables|Default|GetBPac_Dialogue_NonInteractive) "NewEnumerator0") ; Add some condition for your scene
  ))

(event EventBeginPlay
  ;[1 1 1] Begin
  (Variables|/Game/Luxuanlin/DialogueSystem/ActorComponent_Dialogue/BPac_Dialogue_NonInteractive.BPac_Dialogue_NonInteractive_C|SetNPC_Mesh (Variables|Default|GetBPac_Dialogue_NonInteractive) (Variables|Default|GetSkeletalMesh))
  (Variables|Default|SetSaveScene "Scene1.0"))

(event EventStartDialogue(Non-Interactive)
  (params (Action :type ENonIteractiveAction%20Enum :default "NewEnumerator0"))
  ;[1 1 1] Example of a scene dialogue flow
  (switch Utilities|FlowControl|Switch|SwitchonENonIteractiveAction Action
    (:NewEnumerator0
      (bind _returnvalue (Utilities|GetDataTableRow "/Game/Luxuanlin/DialogueSystem/Characters/DataTable/DT_DialogueAnim_A.DT_DialogueAnim_A" (Variables|Default|GetSaveScene))
        (:then
          (Default|PlayAnimandVoice (Variables|Default|GetBPac_Dialogue_NonInteractive) _returnvalue)
          (bind _returnvalue_2 (Utilities|GetDataTableRow "/Game/Luxuanlin/DialogueSystem/Characters/DataTable/DT_Dialogue_A.DT_Dialogue_A" (Variables|Default|GetSaveScene))
            (:then
              (Default|DisplayText (Variables|/Game/Luxuanlin/DialogueSystem/ActorComponent_Dialogue/BPac_Dialogue_NonInteractive.BPac_Dialogue_NonInteractive_C|GetDialogueNonInteractiveUI (Variables|Default|GetBPac_Dialogue_NonInteractive)) _returnvalue_2))))))))

(event EventFinishedDialogue(Non-Interactive)
  ;[1 1 1] Example of a finish dialogue
  (bind _returnvalue (Class|DataTableFunctionLibrary|DoesDataTableRowExist "/Game/Luxuanlin/DialogueSystem/Characters/DataTable/DT_Dialogue_A.DT_Dialogue_A" (Utilities|String|StringToName (Utilities|String|BuildString(Integer) (.LeftS (Utilities|String|Split (Utilities|String|ToString(Name) (Variables|Default|GetSaveScene)) "." "IgnoreCase" "FromEnd")) "." (+ (Math|Conversions|ToInteger(Byte) (.RightS (Utilities|String|Split (Utilities|String|ToString(Name) (Variables|Default|GetSaveScene)) "." "IgnoreCase" "FromEnd"))) 1)))))
  (if _returnvalue
    (Variables|Default|SetSaveScene (Utilities|String|StringToName (Utilities|String|BuildString(Integer) (.LeftS (Utilities|String|Split (Utilities|String|ToString(Name) (Variables|Default|GetSaveScene)) "." "IgnoreCase" "FromEnd")) "." (+ (Math|Conversions|ToInteger(Byte) (.RightS (Utilities|String|Split (Utilities|String|ToString(Name) (Variables|Default|GetSaveScene)) "." "IgnoreCase" "FromEnd"))) 1))))
    (Default|StartSelfTalk(Non-Interactive) (Variables|Default|GetBPac_Dialogue_NonInteractive) "NewEnumerator0")
    (else
      (switch name (Variables|Default|GetSaveScene)
        (:Scene1.9
          (Variables|Default|SetSaveScene "None"))))))

(fn ConstructionScript)

(fn GetInteractType
  (return (Variables|Default|GetInteract%20Type)))