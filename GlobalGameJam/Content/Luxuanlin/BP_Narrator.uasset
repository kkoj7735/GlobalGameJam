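; Narrator Blueprint that plays non-interactive voice and text dialogue for intro, win, lose, die and end scenes through BPacDialogueNonInteractive.
; SaveScene names the current "SceneX.N" row in the narrator voice and text DataTables; finishing a line increments N and replays while rows exist.
; Jump events switch scenes, with JumpToWin advancing its own WinScene row on each call.
; Specific lines fire start, end and big-enemy triggers, and Scene1's end fires the branch trigger.
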(event Custom|JumpToEnd
  ;[1 1 1] Example of a scene dialogue flow
  (Variables|Default|SetSaveScene "Scene5.0")
  (Default|StartSelfTalk(Non-Interactive) (Variables|Default|GetBPac_Dialogue_NonInteractive) "NewEnumerator0"))

(event Custom|JumpToLose
  ;[1 1 1] Example of a scene dialogue flow
  (Variables|Default|SetSaveScene "Scene3.0")
  (Default|StartSelfTalk(Non-Interactive) (Variables|Default|GetBPac_Dialogue_NonInteractive) "NewEnumerator0"))

(event Custom|JumpToWin
  ;[1 1 1] Example of a scene dialogue flow
  (Variables|Default|SetSaveScene (Variables|Default|GetWinScene))
  (Variables|Default|SetWinScene (Utilities|String|StringToName (Utilities|String|BuildString(Integer) (.LeftS (Utilities|String|Split (Utilities|String|ToString(Name) (Variables|Default|GetWinScene)) "." "IgnoreCase" "FromEnd")) "." (+ (Math|Conversions|ToInteger(Byte) (.RightS (Utilities|String|Split (Utilities|String|ToString(Name) (Variables|Default|GetWinScene)) "." "IgnoreCase" "FromEnd"))) 1))))
  (Default|StartSelfTalk(Non-Interactive) (Variables|Default|GetBPac_Dialogue_NonInteractive) "NewEnumerator0"))

(event Custom|NextDialogue
  ;[1 1 1] Example of a scene dialogue flow
  (Default|StartSelfTalk(Non-Interactive) (Variables|Default|GetBPac_Dialogue_NonInteractive) "NewEnumerator0") ; Add some condition for your scene
)

(event Custom|JumpToDie
  ;[1 1 1] Example of a scene dialogue flow
  (Variables|Default|SetSaveScene "Scene4.0")
  (Default|StartSelfTalk(Non-Interactive) (Variables|Default|GetBPac_Dialogue_NonInteractive) "NewEnumerator0"))

(event EventBeginPlay
  ;[1 1 1] Begin
  (Variables|/Game/Luxuanlin/DialogueSystem/ActorComponent_Dialogue/BPac_Dialogue_NonInteractive.BPac_Dialogue_NonInteractive_C|SetNPC_Mesh (Variables|Default|GetBPac_Dialogue_NonInteractive) 0)
  (Variables|Default|SetSaveScene "Scene1.0"))

(event EventStartDialogue(Non-Interactive)
  (params (Action :type ENonIteractiveAction%20Enum :default "NewEnumerator0"))
  (bind _savescene (Variables|Default|GetSaveScene))
  ;[1 1 1] Example of a scene dialogue flow
  (Development|PrintString (Utilities|String|ToString(Name) _savescene))
  (switch Utilities|FlowControl|Switch|SwitchonENonIteractiveAction Action
    (:NewEnumerator0
      (bind _returnvalue (Utilities|GetDataTableRow "/Game/Luxuanlin/DT_DialogueVoice_narrator1.DT_DialogueVoice_narrator1" _savescene)
        (:then
          (Default|PlayAnimandVoice (Variables|Default|GetBPac_Dialogue_NonInteractive) _returnvalue)
          (bind _returnvalue_2 (Utilities|GetDataTableRow "/Game/Luxuanlin/DT_Dialogue_narrator1.DT_Dialogue_narrator1" (Variables|Default|GetSaveScene))
            (:then
              (Default|DisplayText (Variables|/Game/Luxuanlin/DialogueSystem/ActorComponent_Dialogue/BPac_Dialogue_NonInteractive.BPac_Dialogue_NonInteractive_C|GetDialogueNonInteractiveUI (Variables|Default|GetBPac_Dialogue_NonInteractive)) _returnvalue_2))))))))

(event EventFinishedDialogue(Non-Interactive)
  ;[1 1 1] Example of a finish dialogue
  (bind _returnvalue (Class|DataTableFunctionLibrary|DoesDataTableRowExist "/Game/Luxuanlin/DT_Dialogue_narrator1.DT_Dialogue_narrator1" (Utilities|String|StringToName (Utilities|String|BuildString(Integer) (.LeftS (Utilities|String|Split (Utilities|String|ToString(Name) (Variables|Default|GetSaveScene)) "." "IgnoreCase" "FromEnd")) "." (+ (Math|Conversions|ToInteger(Byte) (.RightS (Utilities|String|Split (Utilities|String|ToString(Name) (Variables|Default|GetSaveScene)) "." "IgnoreCase" "FromEnd"))) 1)))))
  (if _returnvalue
    (Variables|Default|SetSaveScene (Utilities|String|StringToName (Utilities|String|BuildString(Integer) (.LeftS (Utilities|String|Split (Utilities|String|ToString(Name) (Variables|Default|GetSaveScene)) "." "IgnoreCase" "FromEnd")) "." (+ (Math|Conversions|ToInteger(Byte) (.RightS (Utilities|String|Split (Utilities|String|ToString(Name) (Variables|Default|GetSaveScene)) "." "IgnoreCase" "FromEnd"))) 1))))
    (if (== (Variables|Default|GetSaveScene) "Scene1.2")
      (Default|CallStartTrigger))
    (if (== (Variables|Default|GetSaveScene) "Scene4.3")
      (Default|CallEndTrigger))
    (if (== (Variables|Default|GetSaveScene) "Scene2.2")
      (Default|CallBigEnemyTrigger))
    (Utilities|FlowControl|Delay 1.0)
    (Default|StartSelfTalk(Non-Interactive) (Variables|Default|GetBPac_Dialogue_NonInteractive) "NewEnumerator0")
    (elif (== (.LeftS (Utilities|String|Split (Utilities|String|ToString(Name) (Variables|Default|GetSaveScene)) "." "IgnoreCase" "FromEnd")) "Scene1")
      (Default|CallBranchTrigger))))

(fn ConstructionScript)

(fn GetInteractType
  (return (Variables|Default|GetInteract%20Type)))