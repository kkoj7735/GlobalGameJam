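; BP_MusicTrack is a rhythm-game track that judges incoming BP_MusicPoint notes as Good, Perfect or Miss.
; Overlapping Good, Perfect and Miss boxes update the pending grade, and ChangePerformance inverts it so letting notes pass scores Perfect.
; PlayClickPoint or the Miss box destroys the current note and spawns a colored BP_Performance readout; clicks also flash cube materials.
; Note-spawning nodes are left unconnected.
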(event OnComponentBeginOverlap(MissBox)
  (params (OverlappedComponent :type Primitive%20Component%20Object%20Reference) (OtherActor :type Actor%20Object%20Reference) (OtherComp :type Primitive%20Component%20Object%20Reference) (OtherBodyIndex :type Integer) (bFromSweep :type Boolean) (SweepResult :type Hit%20Result%20Structure%20%28by%20ref%29))
  (bind _current_point (Variables|Default|GetCurrent%20Point))
  ;[1 1 1] Miss判断
  (if (== OtherActor _current_point)
    (if (Variables|Default|GetChangePerformance)
      ;;[1 0.4556 0.3051] 反转判断：Perfect
      (Variables|Default|SetPerformance "Perfect")
      (Variables|Default|SetTextColor (Class|KismetMathLibrary|LinearColortoRGBE "(R=1.000000,G=0.884920,B=0.116546,A=1.000000)"))
      (else
        (Variables|Default|SetPerformance "Miss")
        (Variables|Default|SetTextColor (Class|KismetMathLibrary|LinearColortoRGBE "(R=1.000000,G=0.014152,B=0.123819,A=1.000000)"))))
    (Actor|DestroyActor _current_point)
    (bind _returnvalue (Game|SpawnActorfromClass "/Game/Dongjingyuan/Blueprints/BP_Performance.BP_Performance_C" (Math|Transform|MakeTransform (Transformation|GetWorldLocation (Variables|Default|GetPerformanceArrow)) "0, 0, 0" "1.000000,1.000000,1.000000") "Undefined" "MultiplyWithRoot" 0 0))
    (bind _output_get (Variables|Default|SetCurrentPerformance _returnvalue))
    (Default|SpawnPerformance _output_get (Variables|Default|GetPerformance) (Variables|Default|GetTextColor))))

(event OnComponentBeginOverlap(perfectBox)
  (params (OverlappedComponent :type Primitive%20Component%20Object%20Reference) (OtherActor :type Actor%20Object%20Reference) (OtherComp :type Primitive%20Component%20Object%20Reference) (OtherBodyIndex :type Integer) (bFromSweep :type Boolean) (SweepResult :type Hit%20Result%20Structure%20%28by%20ref%29))
  ;[1 1 1] Perfect判断
  (if (== OtherActor (Variables|Default|GetCurrent%20Point))
    (if (Variables|Default|GetChangePerformance)
      ;[1 0.4556 0.3051] 反转判断：失败
      (Variables|Default|SetPerformance "Miss")
      (Variables|Default|SetTextColor (Class|KismetMathLibrary|LinearColortoRGBE "(R=1.000000,G=0.014152,B=0.123819,A=1.000000)"))
      (else
        (Variables|Default|SetPerformance "Perfect")
        (Variables|Default|SetTextColor (Class|KismetMathLibrary|LinearColortoRGBE "(R=1.000000,G=0.884920,B=0.116546,A=1.000000)"))))))

(event OnComponentBeginOverlap(GoodBox)
  (params (OverlappedComponent :type Primitive%20Component%20Object%20Reference) (OtherActor :type Actor%20Object%20Reference) (OtherComp :type Primitive%20Component%20Object%20Reference) (OtherBodyIndex :type Integer) (bFromSweep :type Boolean) (SweepResult :type Hit%20Result%20Structure%20%28by%20ref%29))
  ;[1 1 1] Good判断
  (bind _output_get (Variables|Default|SetCurrent%20Point OtherActor))
  (Utilities|Casting|CastToBP_MusicPoint _output_get)
  (if (Variables|Default|GetChangePerformance)
    ;[1 0.4556 0.3051] 反转判断：失败
    (Variables|Default|SetPerformance "Miss")
    (Variables|Default|SetTextColor (Class|KismetMathLibrary|LinearColortoRGBE "(R=1.000000,G=0.014152,B=0.123819,A=1.000000)"))
    (else
      (Variables|Default|SetPerformance "Good")
      (Variables|Default|SetTextColor (Class|KismetMathLibrary|LinearColortoRGBE "(R=0.000000,G=1.000000,B=0.037500,A=1.000000)")))))

(event Custom|PlayClickPoint
  (bind _current_point (Variables|Default|GetCurrent%20Point))
  ;[1 1 1] 按键判断并输出Performance
  (Utilities|IsValid _current_point
    (:Is%20Valid
      (Actor|DestroyActor _current_point)
      (bind _returnvalue (Game|SpawnActorfromClass "/Game/Dongjingyuan/Blueprints/BP_Performance.BP_Performance_C" (Math|Transform|MakeTransform (Transformation|GetWorldLocation (Variables|Default|GetPerformanceArrow)) "0, 0, 0" "1.000000,1.000000,1.000000") "Undefined" "MultiplyWithRoot" 0 0))
      (bind _output_get (Variables|Default|SetCurrentPerformance _returnvalue))
      (Default|SpawnPerformance _output_get (Variables|Default|GetPerformance) (Variables|Default|GetTextColor))
      ;[1 1 1] 改变材质
      (Rendering|Material|SetMaterial (Variables|Default|GetPerfectCube) 0 "/Engine/EditorMaterials/Utilities/LinearColorPicker_MATInst.LinearColorPicker_MATInst")
      (Rendering|Material|SetMaterial (Variables|Default|GetCube) 0 "/Engine/EngineMaterials/BlinkingCaret.BlinkingCaret")
      (Utilities|FlowControl|Delay 0.2)
      (Rendering|Material|SetMaterial (Variables|Default|GetPerfectCube) 0 "/Engine/MapTemplates/Materials/BasicAsset01.BasicAsset01")
      (Rendering|Material|SetMaterial (Variables|Default|GetCube) 0 "/Engine/EngineMaterials/WorldGridMaterial.WorldGridMaterial"))
    (:Is%20Not%20Valid
      (Development|PrintString "Noyet"))))

(event EventTick
  (params (DeltaSeconds :type Float%20%28single-precision%29))
  ;[1 1 1] MusicPoint生成
)

(fn ConstructionScript)