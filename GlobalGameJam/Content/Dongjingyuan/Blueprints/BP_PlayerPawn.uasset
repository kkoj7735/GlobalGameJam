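; BP_PlayerPawn is the player pawn for what appears to be a lane-based music game, switching between three tracks and triggering click points.
; Enhanced Input up/down actions call ChangeTrack, which uses a timeline to lerp the pawn's Y to the clamped target lane.
; A box overlap stores the current BP_MusicTrack, whose PlayClickPoint runs on click input.
; Damage reduces Health and fires event triggers, including a death trigger at exactly zero.
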(event OnComponentBeginOverlap(Box)
  (params (OverlappedComponent :type Primitive%20Component%20Object%20Reference) (OtherActor :type Actor%20Object%20Reference) (OtherComp :type Primitive%20Component%20Object%20Reference) (OtherBodyIndex :type Integer) (bFromSweep :type Boolean) (SweepResult :type Hit%20Result%20Structure%20%28by%20ref%29))
  (bind _asbp_music_track (Utilities|Casting|CastToBP_MusicTrack OtherActor))
  (Variables|Default|SetCurrent%20Track _asbp_music_track))

(event Custom|TakeDamage
  (params (Damage :type Float%20%28double-precision%29))
  (Variables|Default|SetHealth (- (Variables|Default|GetHealth) Damage))
  (Default|CallOnEventTrigger)
  (if (== (Variables|Default|GetHealth) 0.0)
    (Default|CallDeathTrigger)))

(event Custom|Change%20Track
  (params (A :type Integer))
  (bind _returnvalue (Transformation|GetActorLocation))
  (bind (_x _y _z) (Math|Vector|BreakVector _returnvalue))
  ;[1 1 1] 按键选择轨道
  (Variables|Default|SetTarget%20Lane%20Index (Math|Integer|Clamp(Integer) (+ A (Variables|Default|GetCurrent%20Lane%20Index)) 0 2))
  (Variables|Default|SetCurrent%20Y%20Position (.Y (Math|Vector|BreakVector (Transformation|GetActorLocation))))
  (bind _newtrack_2 (Timeline|Timeline PlayFromStart)
    (:Update
      (Transformation|SetActorLocation (Math|Vector|MakeVector _x (Math|Float|Lerp (Variables|Default|GetCurrent%20Y%20Position) (Utilities|Array|Get(acopy) (Variables|Default|GetTrackPosition) (Variables|Default|GetTarget%20Lane%20Index)) _newtrack_2) _z) false false))
    (:Finished
      (Variables|Default|SetCurrent%20Lane%20Index (Variables|Default|GetTarget%20Lane%20Index)))))

(event Input|EnhancedActionEvents|EnhancedInputActionUP_IA
  (params (ActionValue :type Boolean) (ElapsedSeconds :type Float%20%28double-precision%29) (TriggeredSeconds :type Float%20%28double-precision%29) (InputAction :type Input%20Action%20Object%20Reference :default "/Game/Dongjingyuan/Input/UP_IA.UP_IA"))
  ;[1 1 1] 按键选择轨道
  (:Started
    (CallFunction|ChangeTrack -1)))

(event Input|EnhancedActionEvents|EnhancedInputActionDown_IA
  (params (ActionValue :type Boolean) (ElapsedSeconds :type Float%20%28double-precision%29) (TriggeredSeconds :type Float%20%28double-precision%29) (InputAction :type Input%20Action%20Object%20Reference :default "/Game/Dongjingyuan/Input/Down_IA.Down_IA"))
  ;[1 1 1] 按键选择轨道
  (:Started
    (CallFunction|ChangeTrack 1)))

(event Input|EnhancedActionEvents|EnhancedInputActionClick_IA
  (params (ActionValue :type Boolean) (ElapsedSeconds :type Float%20%28double-precision%29) (TriggeredSeconds :type Float%20%28double-precision%29) (InputAction :type Input%20Action%20Object%20Reference :default "/Game/Dongjingyuan/Input/Click_IA.Click_IA"))
  (:Started
    (Default|PlayClickPoint (Variables|Default|GetCurrent%20Track))))

(event EventBeginPlay
  ;[1 1 1] 增强输入映射|Add Input Mapping
  (bind _as玩家控制器 (Utilities|Casting|CastToPlayerController (Pawn|GetController)))
  (Utilities|IsValid (PlayerController|LocalPlayerSubsystems|GetEnhancedInputLocalPlayerSubsystem _as玩家控制器)
    (:Is%20Valid
      (Input|AddMappingContext (PlayerController|LocalPlayerSubsystems|GetEnhancedInputLocalPlayerSubsystem _as玩家控制器) "/Game/Dongjingyuan/Input/IMC_Control.IMC_Control" 0 "(bIgnoreAllPressedKeysUntilRelease=True,bForceImmediately=False)"))))

(fn ConstructionScript)