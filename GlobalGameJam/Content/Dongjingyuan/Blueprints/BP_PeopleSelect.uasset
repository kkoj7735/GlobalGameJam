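; BP_PeopleSelect is a key-controlled selector that switches between three lanes and triggers music tracks.
; Q, W and E each pick a lane index, and ChangeTrack uses a Timeline to lerp the actor's Y position from its current value to that lane's TrackPosition entry.
; When its Box begins overlapping a BP_MusicTrack, it stores that actor as CurrentTrack and calls PlayClickPoint on it.
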(event OnComponentBeginOverlap(Box)
  (params (OverlappedComponent :type Primitive%20Component%20Object%20Reference) (OtherActor :type Actor%20Object%20Reference) (OtherComp :type Primitive%20Component%20Object%20Reference) (OtherBodyIndex :type Integer) (bFromSweep :type Boolean) (SweepResult :type Hit%20Result%20Structure%20%28by%20ref%29))
  (bind _output_get (Variables|Default|SetCurrent%20Track OtherActor))
  (bind _asbp_music_track (Utilities|Casting|CastToBP_MusicTrack _output_get))
  (Default|PlayClickPoint _asbp_music_track))

(event Custom|Change%20Track
  (params (A :type Integer))
  (bind _returnvalue (Transformation|GetActorLocation))
  (bind (_x _y _z) (Math|Vector|BreakVector _returnvalue))
  ;[1 1 1] 按键选择轨道
  (Variables|Default|SetTarget%20Lane%20Index A)
  (Variables|Default|SetCurrent%20Y%20Position (.Y (Math|Vector|BreakVector (Transformation|GetActorLocation))))
  (bind _newtrack_2 (Timeline|Timeline PlayFromStart)
    (:Update
      (Transformation|SetActorLocation (Math|Vector|MakeVector _x (Math|Float|Lerp (Variables|Default|GetCurrent%20Y%20Position) (Utilities|Array|Get(acopy) (Variables|Default|GetTrackPosition) (Variables|Default|GetTarget%20Lane%20Index)) _newtrack_2) _z) false false))))

(event Input|KeyboardEvents|Q
  (params (Key :type Key%20Structure :default "None"))
  ;[1 1 1] 按键选择轨道
  (:Pressed
    (CallFunction|ChangeTrack)))

(event Input|KeyboardEvents|W
  (params (Key :type Key%20Structure :default "None"))
  ;[1 1 1] 按键选择轨道
  (:Pressed
    (CallFunction|ChangeTrack 1)))

(event Input|KeyboardEvents|E
  (params (Key :type Key%20Structure :default "None"))
  ;[1 1 1] 按键选择轨道
  (:Pressed
    (CallFunction|ChangeTrack 2)))

(fn ConstructionScript)