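; BP_SpawnPoint is a timed spawner that places BP_MusicPoint actors at its Arrow's transform, apparently following a music timeline.
; While Start is true, Tick accumulates CurrentTime, clamped to MusicLength, and compares it with the current entry in the PutPoint time array.
; Reaching that time spawns a point and advances the index through a DoOnce, which re-arms only when CurrentTime is below the next entry.
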(event Custom|SpawnPoint
  ;[1 1 1] 按时间生成MusicPoint
  (if (>= (Variables|Default|GetCurrentTime) (Utilities|Array|Get(acopy) (Variables|Default|GetPutPoint) (Variables|Default|GetCurrentPointIndex)))
    (Utilities|FlowControl|DoOnce false :!label _label
      (:Completed
        (Game|SpawnActorfromClass "/Game/Dongjingyuan/Blueprints/BP_MusicPoint.BP_MusicPoint_C" (Transformation|GetWorldTransform (Variables|Default|GetArrow)) "Undefined" "MultiplyWithRoot" 0 0)
        (Math|Integer|IncrementInt (Variables|Default|GetCurrentPointIndex))))
    (else
      (goto _label Reset))))

(event Custom|CountTime
  ;[1 1 1] 计算时间
  (bind _output_get (Variables|Default|SetCurrentTime (Math|Float|Clamp(Float) (+ (Variables|Default|GetCurrentTime) (Utilities|Time|GetWorldDeltaSeconds)) 0.0 (Variables|Default|GetMusicLength)))))

(event Custom|SpawnAtTime)

(event EventTick
  (params (DeltaSeconds :type Float%20%28single-precision%29))
  ;[1 1 1] 音乐长度判断
  (if (Variables|Default|GetStart)
    (CallFunction|CountTime)
    (if (not (> (Variables|Default|GetCurrentPointIndex) (Utilities|Array|Length (Variables|Default|GetPutPoint))))
      (CallFunction|SpawnPoint))))

(fn ConstructionScript)